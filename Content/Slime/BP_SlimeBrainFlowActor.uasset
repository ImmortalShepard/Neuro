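; Actor that drives a slime simulation with BrainFlow brain data from the NeuroGameMode.
; Each tick it rate-limits changes in the channel values, falling back to four channels from a BrainFlow table actor when live data fails.
; Each species takes the channel at its index to offset base move speed, with a minimum, and wrap color hue before updating the slime sim actor.
; It also prints raw data periodically.
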(event EventBeginPlay
  (bind _asneuro_game_mode (Utilities|Casting|CastToNeuroGameMode (Game|GetGameMode)))
  (bind _output_get (Variables|Default|SetNeuro%20Game%20Mode _asneuro_game_mode))
  (bind _returnvalue (Class|NeuroGameMode|GetBrainFlowSize _output_get))
  (Utilities|Array|Resize (Variables|Default|GetBrainFlowData) _returnvalue))

(event EventTick
  (params (DeltaSeconds :type Float%20%28single-precision%29))
  (bind _slimesimactor (Variables|Default|GetSlimeSimActor))
  (bind _slimesettings (Variables|/Script/SlimeComputeShaderDeclaration.SlimeSimActor|GetSlimeSettings _slimesimactor))
  (CallFunction|PrintRawData DeltaSeconds)
  (bind _brainflowdata (CallFunction|GetBrainFlowData))
  (for (_array_element _array_index) _brainflowdata
    (Utilities|Array|SetArrayElem (Variables|Default|GetBrainFlowData) _array_index (CallFunction|MovetoValue (Utilities|Array|Get(acopy) (Variables|Default|GetBrainFlowData) _array_index) _array_element (* (Variables|Default|GetBrainFlowChange) DeltaSeconds)) true))
  (bind _output_get (Variables|Default|SetSpecies%20Settings (Variables|/Script/SlimeComputeShaderDeclaration.SlimeSettings|GetSpeciesSettings _slimesettings)))
  (Variables|Default|SetBounds%20Settings (Variables|/Script/SlimeComputeShaderDeclaration.SlimeSettings|GetBoundsSettings _slimesettings))
  (for _index (range 0 (- (Utilities|Array|Length _output_get) 1))
    (CallFunction|ProcessBrainData _index))
  (Class|SlimeSimActor|UpdateSlimeSim (Variables|Default|GetSlimeSimActor) (Variables|Default|GetSpecies%20Settings) (Variables|Default|GetBounds%20Settings)))

(fn ConstructionScript)

(fn ProcessBrainData
  (params (Index :type Integer))
  (bind _brainflowdata (Variables|Default|GetBrainFlowData))
  (bind _species_settings (Variables|Default|GetSpecies%20Settings))
  (bind _output (Utilities|Array|Get(acopy) _species_settings Index))
  (bind _output_2 (Utilities|Array|Get(acopy) _brainflowdata Index))
  (bind _speciessettings (Utilities|Struct|BreakSlimeSpeciesSettings _output))
  (bind (_movespeed _turnspeed _sensorangledegrees _sensoroffsetdst _sensorsize _color) (Utilities|Struct|BreakSpeciesSettings _speciessettings))
  (bind (_h _s _v _a) (Math|Color|RGBtoHSV(LinearColor) _color))
  (Utilities|Struct|SetmembersinSpeciesSettings _speciessettings (Math|Float|Max(Float) (+ _movespeed (* (Variables|Default|GetSpeedModifier) _output_2)) (Variables|Default|GetMinSpeed)) (Class|KismetMathLibrary|HSVtoRGB (CallFunction|ClampHue (+ _h (* _output_2 (Variables|Default|GetHueChange)))) _s _v _a)))

(fn MovetoValue
  (params (OldValue :type Float%20%28single-precision%29) (NewValue :type Float%20%28single-precision%29) (MaxChange :type Float%20%28single-precision%29))
  (bind _returnvalue (- NewValue OldValue))
  (if (<= (Math|Float|Absolute(Float) _returnvalue) MaxChange)
    (return NewValue)
    (else
      (return (+ OldValue (* (Math|Float|Sign(Float) _returnvalue) MaxChange))))))

(fn ClampHue
  (params (Hue :type Float%20%28single-precision%29))
  (return (- Hue (* (Math|Float|Floor (/ Hue 3.6e+02)) 3.6e+02))))

(fn PrintRawData
  (params (DeltaTime :type Float%20%28single-precision%29))
  (if (<= (Variables|Default|GetTimer) 0.0)
    (Variables|Default|SetTimer (Variables|Default|GetPrintInterval))
    (Variables|Default|SetIn%20String "")
    (bind _rawbrainflowdata (Class|NeuroGameMode|GetRawBrainFlowData (Variables|Default|GetNeuro%20Game%20Mode))
      (:True
        _)
      (:False
        _))
    (for _array_element _rawbrainflowdata
      (Variables|Default|SetIn%20String (Utilities|String|Append (Utilities|String|Append (Variables|Default|GetIn%20String) (Utilities|String|ToString(Float) _array_element)) ", ")))
    (Development|PrintString (Variables|Default|GetIn%20String) true true "(R=0.000000,G=0.660000,B=1.000000,A=1.000000)" (Math|Float|Max(Float) (- (Variables|Default|GetPrintInterval) 0.1) 0.1))
    (else
      (Variables|Default|SetTimer (- (Variables|Default|GetTimer) DeltaTime))))
  (return))

(fn GetBrainFlowData
  (bind _brainflowdata (Class|NeuroGameMode|GetBrainFlowData (Variables|Default|GetNeuro%20Game%20Mode))
    (:True
      (return _brainflowdata))
    (:False
      (bind _returnvalue (Class|BrainFlowTableActor|GetBrainFlowData (Variables|Default|GetBrainFlowTableActor)))
      (return (Utilities|Array|MakeArray (.a2 _returnvalue) (.a1 _returnvalue) (.c4 _returnvalue) (.c3 _returnvalue))))))