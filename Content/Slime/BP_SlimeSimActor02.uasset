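; Slime simulation actor that modulates its species with live BrainFlow data from the NeuroGameMode.
; When the game mode has no data, it reads four channels from a BrainFlow table actor instead.
; Each tick, a channel pair per species offsets the SlimeSettings move speed, wrapped color hue and decay rate, then updates the sim.
; Releasing the Exit input opens the start level.
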(event EventBeginPlay
  (bind _asneuro_game_mode (Utilities|Casting|CastToNeuroGameMode (Game|GetGameMode)))
  (Variables|Default|SetNeuro%20Game%20Mode _asneuro_game_mode))

(event EventTick
  (params (DeltaSeconds :type Float%20%28single-precision%29))
  (CallFunction|UpdateSpeciesSettings))

(event Input|ActionEvents|InputActionExit
  (params (Key :type Key%20Structure :default "None"))
  (:Released
    (Game|OpenLevel(byObjectReference) "/Game/Levels/StartLevel.StartLevel")))

(fn ConstructionScript)

(fn GetBrainFlowData
  (bind _brainflowdata (Class|NeuroGameMode|GetBrainFlowData (Variables|Default|GetNeuro%20Game%20Mode))
    (:True
      (return _brainflowdata))
    (:False
      (bind _returnvalue (Class|BrainFlowTableActor|GetBrainFlowData (Variables|Default|GetBrainFlowTableActor)))
      (return (Utilities|Array|MakeArray (.a2 _returnvalue) (.a1 _returnvalue) (.c4 _returnvalue) (.c3 _returnvalue))))))

(fn UpdateSpeciesSettings
  (Variables|Default|SetSpecies%20Settings (Variables|/Script/SlimeComputeShaderDeclaration.SlimeSettings|GetSpeciesSettings (Variables|Default|GetSlimeSettings)))
  (bind _brainflowdata (CallFunction|GetBrainFlowData))
  (for (_ _array_index) (Variables|Default|GetSpecies%20Settings)
    (Utilities|Struct|SetmembersinSlimeSpeciesSettings (Utilities|Array|Get(acopy) (Variables|Default|GetSpecies%20Settings) _array_index) (+ (* (Utilities|Array|Get(acopy) _brainflowdata (+ (* _array_index 2) 1)) (Variables|Default|GetDecayRateChange)) (.DecayRate (Utilities|Struct|BreakSlimeSpeciesSettings (Utilities|Array|Get(acopy) (Variables|Default|GetSpecies%20Settings) _array_index)))))
    (Utilities|Struct|SetmembersinSpeciesSettings (.SpeciesSettings (Utilities|Struct|BreakSlimeSpeciesSettings (Utilities|Array|Get(acopy) (Variables|Default|GetSpecies%20Settings) _array_index))) (+ (.MoveSpeed (Utilities|Struct|BreakSpeciesSettings (.SpeciesSettings (Utilities|Struct|BreakSlimeSpeciesSettings (Utilities|Array|Get(acopy) (Variables|Default|GetSpecies%20Settings) _array_index))))) (* (Utilities|Array|Get(acopy) _brainflowdata (* _array_index 2)) (Variables|Default|GetMoveSpeedChange))) (Class|KismetMathLibrary|HSVtoRGB (CallFunction|ClampHue (+ (.H (Math|Color|RGBtoHSV(LinearColor) (.Color (Utilities|Struct|BreakSpeciesSettings (.SpeciesSettings (Utilities|Struct|BreakSlimeSpeciesSettings (Utilities|Array|Get(acopy) (Variables|Default|GetSpecies%20Settings) _array_index))))))) (* (Utilities|Array|Get(acopy) _brainflowdata (* _array_index 2)) (Variables|Default|GetHueChange)))) (.S (Math|Color|RGBtoHSV(LinearColor) (.Color (Utilities|Struct|BreakSpeciesSettings (.SpeciesSettings (Utilities|Struct|BreakSlimeSpeciesSettings (Utilities|Array|Get(acopy) (Variables|Default|GetSpecies%20Settings) _array_index))))))) (.V (Math|Color|RGBtoHSV(LinearColor) (.Color (Utilities|Struct|BreakSpeciesSettings (.SpeciesSettings (Utilities|Struct|BreakSlimeSpeciesSettings (Utilities|Array|Get(acopy) (Variables|Default|GetSpecies%20Settings) _array_index))))))) (.A (Math|Color|RGBtoHSV(LinearColor) (.Color (Utilities|Struct|BreakSpeciesSettings (.SpeciesSettings (Utilities|Struct|BreakSlimeSpeciesSettings (Utilities|Array|Get(acopy) (Variables|Default|GetSpecies%20Settings) _array_index))))))))))
  (Class|SlimeSimActor|UpdateSlimeSimSpecies (Variables|Default|GetSpecies%20Settings)))

(fn ClampHue
  (params (Hue :type Float%20%28single-precision%29))
  (return (- Hue (* (Math|Float|Floor (/ Hue 3.6e+02)) 3.6e+02))))