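; BP_ShaderBrainFlowActor feeds BrainFlow data from the game mode into shaders through a material parameter collection.
; BeginPlay caches the NeuroGameMode reference.
; Each Tick fetches the BrainFlow data array and, when the fetch succeeds, writes each element to a scalar parameter in MPC_BrainFlow, named "BrainFlow" plus the element's index.
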(event EventBeginPlay
  (bind _asneuro_game_mode (Utilities|Casting|CastToNeuroGameMode (Game|GetGameMode)))
  (Variables|Default|SetNeuro%20Game%20Mode _asneuro_game_mode))

(event EventTick
  (params (DeltaSeconds :type Float%20%28single-precision%29))
  (bind _brainflowdata (Class|NeuroGameMode|GetBrainFlowData (Variables|Default|GetNeuro%20Game%20Mode))
    (:True
      (for (_array_element _array_index) _brainflowdata
        (Rendering|Material|SetScalarParameterValue "/Game/Shader/MPC_BrainFlow.MPC_BrainFlow" (Utilities|String|StringToName (Utilities|String|Append "BrainFlow" (Utilities|String|ToString(Integer) _array_index))) _array_element :!class /Script/Engine.KismetMaterialLibrary)))))

(fn ConstructionScript)